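; Blueprint function library that supplies shared UI colors read from a Material Parameter Collection.
; GetColorByTier switches on a tier, from None through Royal, reads the vector parameter of the same name and returns it as a Slate color.
; GetButtonBackgroundColor returns the collection's button background parameter as a raw color.
; A Select node and several hardcoded Slate colors remain in the tier graph but are unused.
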(fn GetColorbyTier
  (params (Selection :type EItemTier%20Enum :default "None"))
  (switch Utilities|FlowControl|Switch|SwitchonEItemTier Selection
    (:None
      (bind _returnvalue (Rendering|Material|GetVectorParameterValue 0 (LocalVariables|GetMPC) (Utilities|Name|MakeLiteralName "None") :!class /Script/Engine.KismetMaterialLibrary))
      (return (Utilities|Struct|MakeSlateColor _returnvalue)))
    (:Common
      (bind _returnvalue_2 (Rendering|Material|GetVectorParameterValue 0 (LocalVariables|GetMPC) (Utilities|Name|MakeLiteralName "Common") :!class /Script/Engine.KismetMaterialLibrary))
      (return (Utilities|Struct|MakeSlateColor _returnvalue_2)))
    (:Uncommon
      (bind _returnvalue_3 (Rendering|Material|GetVectorParameterValue 0 (LocalVariables|GetMPC) (Utilities|Name|MakeLiteralName "Uncommon") :!class /Script/Engine.KismetMaterialLibrary))
      (return (Utilities|Struct|MakeSlateColor _returnvalue_3)))
    (:Rare
      (bind _returnvalue_4 (Rendering|Material|GetVectorParameterValue 0 (LocalVariables|GetMPC) (Utilities|Name|MakeLiteralName "Rare") :!class /Script/Engine.KismetMaterialLibrary))
      (return (Utilities|Struct|MakeSlateColor _returnvalue_4)))
    (:Epic
      (bind _returnvalue_5 (Rendering|Material|GetVectorParameterValue 0 (LocalVariables|GetMPC) (Utilities|Name|MakeLiteralName "Epic") :!class /Script/Engine.KismetMaterialLibrary))
      (return (Utilities|Struct|MakeSlateColor _returnvalue_5)))
    (:Royal
      (bind _returnvalue_6 (Rendering|Material|GetVectorParameterValue 0 (LocalVariables|GetMPC) (Utilities|Name|MakeLiteralName "Royal") :!class /Script/Engine.KismetMaterialLibrary))
      (return (Utilities|Struct|MakeSlateColor _returnvalue_6)))))

(fn GetButtonBackgroundColor
  (bind _returnvalue (Rendering|Material|GetVectorParameterValue 0 (LocalVariables|GetMPC) (Utilities|Name|MakeLiteralName "ButtonBackground") :!class /Script/Engine.KismetMaterialLibrary))
  (return _returnvalue))