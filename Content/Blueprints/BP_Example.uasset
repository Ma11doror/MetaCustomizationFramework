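; Example Blueprint that exercises an InventoryComponent with a set of "type two" clothing items.
; One second after BeginPlay, it adds boots, shorts, a hoody, jeans and flip-flops to the inventory.
; Disconnected chains, which never run, hold timed tests for equipping items by literal name and for removing boots through a negative AddItem count.
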(event EventBeginPlay
  (bind _inventorycomponent (Variables|Default|GetInventoryComponent))
  (Utilities|FlowControl|Delay 1.0)
  (Class|InventoryComponent|AddItem (Variables|Default|GetInventoryComponent) "/Game/PrimaryAssets/Items/TypeTwo/Boots/w_type_two_boots.w_type_two_boots" 1)
  (Class|InventoryComponent|AddItem (Variables|Default|GetInventoryComponent) "/Game/PrimaryAssets/Items/TypeTwo/Bottom/w_type_two_shorts.w_type_two_shorts" 2)
  (Class|InventoryComponent|AddItem (Variables|Default|GetInventoryComponent) "/Game/PrimaryAssets/Items/TypeTwo/Top/w_type_two_hoody.w_type_two_hoody" 1)
  (Class|InventoryComponent|AddItem _inventorycomponent "/Game/PrimaryAssets/Items/TypeTwo/Bottom/w_type_two_jeans.w_type_two_jeans" 1)
  (Class|InventoryComponent|AddItem _inventorycomponent "/Game/PrimaryAssets/Items/TypeTwo/Boots/w_type_two_flip_flops.w_type_two_flip_flops" 1))

(fn ConstructionScript)